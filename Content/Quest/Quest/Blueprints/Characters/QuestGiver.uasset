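; Quest giver NPC that offers the player a quest through branching dialogue.
; BeginPlay spawns an actor for the quest at its own transform.
; StartDialouge turns it toward the player and opens chained dialogue widgets, each answer event choosing the next, or another widget if the quest was already given.
; Accepting calls GiveQuestToPlayer, which hands over a valid quest once and changes the marker to a question mark.
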(event `self.ReceiveBeginPlay`
  ;[1 1 1] Create Quest
  (`|SpawnActorFromClass` null (`self.GetTransform`) true)
  (set `self.QuestToGive` null))

(event `StartDialouge`
  ;[1 1 1] Look at player
  (`self.SetActorRotation` (`KismetMathLibrary.FindLookAtRotation` (`self.K2_GetActorLocation`) (`self.K2_GetActorLocation` (`GameplayStatics.GetPlayerCharacter` 0))))
  (if (`self.QuestGiven`)
    ;[1 1 1] Player already has received the quest
    (`|CreateWidget` null)
    (`UserWidget.AddToViewport` 0)
    (else
      ;[1 1 1] Show dialouge
      (`|CreateWidget` "/Game/Quest/Quest/UMG/Dialouge.Dialouge_C")
      (`UserWidget.AddToViewport` 0)
      (add `self.Event_Answer` (delegate `Dialouge1`)))))

(event `Dialouge3_Copy` :!signature `self.Event_Answer`
  (params (Answer :type Integer))
  (switch `int` Answer
    (:`1`
      _)
    (:`2`
      _))
  (`|CreateWidget` null)
  (`UserWidget.AddToViewport` 0)
  (add `self.Event_Answer` (delegate `Dialouge4`)))

(event `Dialouge4` :!signature `self.Event_Answer`
  (params (Answer :type Integer))
  (switch `int` Answer
    (:`1`
      ;[1 1 1] Give Quest to Player
      (`self.GiveQuestToPlayer`))
    (:`2`
      (`|CreateWidget` null)
      (`UserWidget.AddToViewport` 0))))

(event `Dialouge1` :!signature `self.Event_Answer`
  (params (Answer :type Integer))
  ;[1 1 1] Show dialouge
  (switch `int` Answer
    (:`1`
      (`|CreateWidget` null)
      (`UserWidget.AddToViewport` 0)
      (add `self.Event_Answer` (delegate `Dialouge3_Copy`)))
    (:`2`
      (`|CreateWidget` null)
      (`UserWidget.AddToViewport` 0)
      (add `self.Event_Answer` (delegate `Dialouge3`)))))

(event `Dialouge3` :!signature `self.Event_Answer`
  (params (Answer :type Integer))
  (switch `int` Answer
    (:`1`
      (`|CreateWidget` null)
      (`UserWidget.AddToViewport` 0))))

(fn `GiveQuestToPlayer`
  ;[1 1 1] Give quest to player
  (cast `` (`GameplayStatics.GetPlayerCharacter` 0))
  (`/Engine/EditorBlueprintResources/StandardMacros.IsValid` null
    (:`Is Valid`
      (`self.GetQuest` null)
      ;[1 1 1] Change to question mark
      (`TextRenderComponent.SetText` (`self.QuestMarker`) "?")
      ;[1 1 1] Quest can be given to the player only once
      (set `self.QuestGiven` true))
    (:`Is Not Valid`
      (`KismetSystemLibrary.PrintString` "No quest to give!"))))

(fn `UserConstructionScript`)